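; Gameplay ability for the Hollow Purple attack, which spawns a BP_HollowPurple actor at the player character after a delay.
; On activation it clears CanViolet on player 0's BP_ThirdPersonCharacter and starts a one-shot twelve-second timer.
; When the timer fires, it spawns the actor slightly above the character with its rotation and scale, prints a French message, restores CanViolet and ends the ability.
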(event Custom|ThrowViolet
  (Game|SpawnActorfromClass "/Game/BP_HollowPurple.BP_HollowPurple_C" (Math|Transform|MakeTransform (+ (.location (Transformation|GetActorTransform (stale Ability|EventActivateAbility _asbp_third_person_character))) "0.000000,0.000000,50.000000") (.rotation (Transformation|GetActorTransform (stale Ability|EventActivateAbility _asbp_third_person_character))) (.scale (Transformation|GetActorTransform (stale Ability|EventActivateAbility _asbp_third_person_character)))) "Undefined" "MultiplyWithRoot" 0 0)
  (Development|PrintString "Mon roi est prêt à detruire Sukuna" true true "(R=1.000000,G=0.656512,B=0.000000,A=1.000000)")
  (Variables|/Game/ThirdPerson/Blueprints/BP_ThirdPersonCharacter.BP_ThirdPersonCharacter_C|SetCanViolet? (stale Ability|EventActivateAbility _asbp_third_person_character) true)
  (Ability|EndAbility))

(event Ability|EventActivateAbility
  (bind _asbp_third_person_character (Utilities|Casting|CastToBP_ThirdPersonCharacter (Game|GetPlayerCharacter 0)))
  (Variables|/Game/ThirdPerson/Blueprints/BP_ThirdPersonCharacter.BP_ThirdPersonCharacter_C|SetCanViolet? _asbp_third_person_character false)
  (Utilities|Time|SetTimerbyEvent (delegate Custom|ThrowViolet) 12.0))